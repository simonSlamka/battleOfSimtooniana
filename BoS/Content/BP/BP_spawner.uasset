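; BP_spawner is a spawner that places a configurable number of AI pawns in a grid at level start.
; On BeginPlay it loops through the count, using a modulo on the index to start a new row every AmountPerRow pawns, stepped by Spacing.
; Each pawn spawns via SpawnAIFromClass with the chosen class and behavior tree, offset from the actor's location, with the first row one spacing along Y.
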(event EventBeginPlay
  (bind _returnvalue (Transformation|GetActorLocation))
  (bind (_x _y _z) (Math|Vector|BreakVector _returnvalue))
  (for _index (range 0 (- (Variables|Default|GetnumToSpawn) 1))
    (if (== (Math|Integer|%(Integer) _index (Variables|Default|GetamountPerRow)) 0)
      (Variables|Default|SetYLoc (+ (Variables|Default|GetYLoc) (Variables|Default|Getspacing)))
      (Variables|Default|SetXLoc 0.0))
    (AI|SpawnAIFromClass (Variables|Default|GetwhichClassToSpawn) (Variables|Default|GetBT) (Math|Vector|MakeVector (+ (Variables|Default|GetXLoc) _x) (+ (Variables|Default|GetYLoc) _y) _z) "0, 0, 0" false 0)
    (Variables|Default|SetXLoc (+ (Variables|Default|GetXLoc) (Variables|Default|Getspacing)))))

(fn ConstructionScript)